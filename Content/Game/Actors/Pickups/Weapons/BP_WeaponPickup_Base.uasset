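; BP_WeaponPickup_Base is a base weapon pickup that grants its WeaponToAdd class to the user who picks it up.
; The construction script sets the Mesh3P skeletal mesh from that class's defaults, so the pickup previews its weapon.
; On pickup, it adds the weapon to the user's inventory only if not already held.
; An invalid class prints an error and disables collision at BeginPlay.
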(event `self.ReceiveBeginPlay`
  (if (not (`KismetSystemLibrary.IsValidClass` (`self.WeaponToAdd`)))
    (`KismetSystemLibrary.PrintString` (`KismetStringLibrary.Concat_StrStr` "ERROR: " (`KismetSystemLibrary.GetDisplayName` self) " will not spawn its pickup class because the WeaponToAdd class is invalid. Please add a class for this to use!") false)
    (`self.SetActorEnableCollision` false)))

(event `self.BlueprintHandlePickup`
  (params (ForUser :type "InfinityCharacter Object Reference"))
  (if (not (`InfinityCharacter.HasItemInInventory` ForUser (`self.WeaponToAdd`)))
    (`InfinityCharacter.AddItemToInventory` ForUser (`self.WeaponToAdd`))))

(fn `UserConstructionScript`
  (if (`KismetSystemLibrary.IsValidClass` (`self.WeaponToAdd`))
    (`SkinnedMeshComponent.SetSkinnedAssetAndUpdate` (`self.Mesh3P`) (defaults `Object` (`self.WeaponToAdd`)) true)))