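; Base pickup actor that grants a power-up to the user who collects it.
; On pickup it passes its configured PowerUpClass to the user's GivePowerUp.
; At BeginPlay it checks that the class is valid, and if not, prints an error and disables its collision.
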(event `self.BlueprintHandlePickup`
  (params (ForUser :type "InfinityCharacter Object Reference"))
  (`InfinityCharacter.GivePowerUp` ForUser (`self.PowerUpClass`)))

(event `self.ReceiveBeginPlay`
  (if (not (`KismetSystemLibrary.IsValidClass` (`self.PowerUpClass`)))
    (`KismetSystemLibrary.PrintString` (`KismetStringLibrary.Concat_StrStr` "ERROR: " (`KismetSystemLibrary.GetDisplayName` self) " has no pickup class. Disabling collision for this actor!") false)
    (`self.SetActorEnableCollision` false)))

(fn `UserConstructionScript`)